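; Prototype black hole actor that pulls in physics-simulating static mesh actors and destroys them.
; A timeline started on BeginPlay scales the attraction force toward its maximum over time.
; Each tick, static mesh actors inside the effect sphere receive a negative radial force with linear falloff, applied as acceleration so mass is ignored.
; Any that overlap the inner destroy sphere are destroyed.
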(event `self.ReceiveBeginPlay`
  (bind (_direction _strength) (`Timeline|Increase Strength` :!via `PlayFromStart`)
    (:`Update`
      (set `self.AttractionForce` (* (`self.MaxAttractionForce`) _strength)))))

(event `self.ReceiveTick`
  (params (DeltaSeconds :type "Float (single-precision)"))
  (for _array_element (`PrimitiveComponent.GetOverlappingActors` (`self.Effect_Radius`) "/Script/Engine.StaticMeshActor")
    (if (`PrimitiveComponent.IsOverlappingActor` (`self.Destroy_Radius`) _array_element)
      (`self.K2_DestroyActor` _array_element)
      (else
        (bind _asstatic_mesh_actor (cast `StaticMeshActor` _array_element))
        (bind _staticmeshcomponent (`StaticMeshActor.StaticMeshComponent` _asstatic_mesh_actor))
        (if (`SceneComponent.IsSimulatingPhysics` _staticmeshcomponent "None")
          (`PrimitiveComponent.AddRadialForce` _staticmeshcomponent (`self.K2_GetActorLocation`) (`SphereComponent.SphereRadius` (`self.Effect_Radius`)) (* (`self.AttractionForce`) -1.0) "RIF_Linear" true))))))

(fn `UserConstructionScript`)